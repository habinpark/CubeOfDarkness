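; BatProjectile_BP is a projectile actor that keeps turning toward the player and damages whatever it hits.
; On BeginPlay it caches the player pawn as CubePlayerPawn_BP and starts FacePlayer, a self-calling event on a very short Delay, used instead of Tick, that interpolates its rotation toward the player.
; On Hit it applies fixed damage to the other actor and destroys itself.
; The graph contains no movement logic.
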(event Custom|FacePlayer
  ;[1 1 1] Always face player
  (Transformation|SetActorRotation (Math|Interpolation|RInterpTo (Transformation|GetActorRotation) (Math|Rotator|FindLookatRotation (Transformation|GetActorLocation) (Transformation|GetActorLocation (Variables|Default|GetCube%20Player%20Pawn%20BP))) (Utilities|Time|GetWorldDeltaSeconds) 2e+01))
  (Utilities|FlowControl|Delay 0.001)
  (CallFunction|FacePlayer))

(event EventBeginPlay
  (bind _ascube_player_pawn_bp (Utilities|Casting|CastToCubePlayerPawn_BP (Game|Player|GetPlayerPawn 0)))
  (Variables|Default|SetCube%20Player%20Pawn%20BP _ascube_player_pawn_bp)
  (CallFunction|FacePlayer))

(event Collision|EventActorBeginOverlap
  (params (OtherActor :type Actor%20Object%20Reference)))

(event EventTick
  (params (DeltaSeconds :type Float%20%28single-precision%29)))

(event Collision|EventHit
  (params (MyComp :type Primitive%20Component%20Object%20Reference) (Other :type Actor%20Object%20Reference) (OtherComp :type Primitive%20Component%20Object%20Reference) (bSelfMoved :type Boolean) (HitLocation :type Vector :default "0, 0, 0") (HitNormal :type Vector :default "0, 0, 0") (NormalImpulse :type Vector :default "0, 0, 0") (Hit :type Hit%20Result%20Structure%20%28by%20ref%29))
  (Game|Damage|ApplyDamage Other 1e+02 0 0)
  (Actor|DestroyActor))

(fn ConstructionScript)